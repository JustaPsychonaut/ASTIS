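; BP_ShipSave stores a ship's layout as data, built from a cabin and its child components.
; SaveShipData records the cabin's class, its DefaultCabin value and a uniform scale vector built from its ScaleValue.
; It clears and refills two parallel arrays with each child component's class and the relative transform of that component's Basement.
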(fn `SaveShipData`
  (params (Cabin :type "/Game/Blueprints/Components/CompParent Object Reference"))
  (bind _returnvalue (`KismetMathLibrary.Conv_IntToDouble` (`/Game/Blueprints/Components/CompParent.ScaleValue` Cabin)))
  (set `self.Scale` (`KismetMathLibrary.MakeVector` _returnvalue _returnvalue _returnvalue))
  (set `self.Cabin` (`GameplayStatics.GetObjectClass` Cabin))
  (`KismetArrayLibrary.Array_Clear` (`self.Comps`))
  (`KismetArrayLibrary.Array_Clear` (`self.RelativeTransforms`))
  (set `self.DefaultCabin` (`/Game/Blueprints/Components/CompParent.DefaultCabin` Cabin))
  (for _array_element (`/Game/Blueprints/Components/CompParent.ChildrenComps` Cabin)
    (`KismetArrayLibrary.Array_Add` (`self.Comps`) (`GameplayStatics.GetObjectClass` _array_element))
    (`KismetArrayLibrary.Array_Add` (`self.RelativeTransforms`) (`SceneComponent.GetRelativeTransform` (`/Game/Blueprints/Components/CompParent.Basement` _array_element))))
  (return))