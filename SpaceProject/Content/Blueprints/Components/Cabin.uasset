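; Cabin is a ship part Blueprint that marks itself as the default and root cabin and can spawn the ship's controller.
; Its construction script runs the parent's, then sets the default flag and root cabin reference.
; SpawnController always spawns a ShipController at the Basement transform, attaches it to the cabin root, calls SpawnDefaultController on it and gives it a back-reference to the cabin.
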(fn `SpawnController`
  (bind _returnvalue (`|SpawnActorFromClass` "/Game/Blueprints/Components/ShipController.ShipController_C" (`SceneComponent.K2_GetComponentToWorld` (`self.Basement`)) "AlwaysSpawn" "OverrideRootScale"))
  (bind _output_get (set `self.Controller` _returnvalue))
  (`SceneComponent.K2_AttachTo` (`self.K2_GetRootComponent` _output_get) (`self.K2_GetRootComponent` self) "None" "KeepRelativeOffset" true)
  (`Pawn.SpawnDefaultController` _output_get)
  (set `/Game/Blueprints/Components/ShipController.Cabin` self _output_get))

(fn `UserConstructionScript`
  (`parent.UserConstructionScript`)
  (set `self.DefaultCabin` true)
  (set `self.RootCabin` self))