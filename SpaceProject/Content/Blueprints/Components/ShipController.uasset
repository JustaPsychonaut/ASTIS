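; Ship flight controller that turns player input into six-axis physics movement of a referenced Cabin's Basement body.
; Axis inputs add linear and angular velocity along the Cabin camera's axes, with thrust scaled by FlyingSpeed.
; Forward thrust eases the camera FOV wider within a clamped range, narrowing it otherwise.
; Pressing G exits the ship by spawning MyPawn1 above it and transferring possession and view.
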(event `InputAxis|ImpulseForward`
  (params (AxisValue :type "Float (single-precision)"))
  (bind _cabin (`self.Cabin`))
  (bind _camera (`/Game/Blueprints/Components/Cabin.Camera` (`self.Cabin`)))
  (bind _fieldofview (`CameraComponent.FieldOfView` _camera))
  (bind _returnvalue (`KismetMathLibrary.Sqrt` (/ (`KismetMathLibrary.Abs` (- 89.0 _fieldofview)) 10.0)))
  ;[1 1 1] Movement
  (`PrimitiveComponent.SetPhysicsLinearVelocity` (`/Game/Blueprints/Components/CompParent.Basement` _cabin) (* (`SceneComponent.GetForwardVector` (`/Game/Blueprints/Components/Cabin.Camera` _cabin)) (* (`self.Flying Speed`) AxisValue)) true "None")
  (if (< 0.0 AxisValue)
    (set `CameraComponent.FieldOfView` (`KismetMathLibrary.FClamp` (+ _fieldofview _returnvalue) 90.0 110.0) _camera)
    (else
      (set `CameraComponent.FieldOfView` (`KismetMathLibrary.FClamp` (- _fieldofview _returnvalue) 90.0 110.0) _camera))))

(event `InputAxis|Jump/FlyUp`
  (params (AxisValue :type "Float (single-precision)"))
  (bind _cabin (`self.Cabin`))
  ;[1 1 1] Movement
  (`PrimitiveComponent.SetPhysicsLinearVelocity` (`/Game/Blueprints/Components/CompParent.Basement` _cabin) (* (`SceneComponent.GetUpVector` (`/Game/Blueprints/Components/Cabin.Camera` _cabin)) (* (`self.Flying Speed`) AxisValue)) true "None"))

(event `Key|G`
  (params (Key :type "Key Structure" :default "AnyKey"))
  (bind _returnvalue (`GameplayStatics.GetPlayerController` 0))
  (bind _basement (`/Game/Blueprints/Components/CompParent.Basement` (`self.Cabin`)))
  (:`Pressed`
    (`Controller.UnPossess` _returnvalue)
    (bind _returnvalue_2 (`|SpawnActorFromClass` "/Game/Blueprints/MyPawn1.MyPawn1_C" (`KismetMathLibrary.MakeTransform` (+ (* (`SceneComponent.GetUpVector` _basement) 300) (`SceneComponent.K2_GetComponentLocation` _basement)) (`SceneComponent.K2_GetComponentRotation` _basement)) "AlwaysSpawn" "OverrideRootScale"))
    (`Controller.Possess` _returnvalue _returnvalue_2)
    (`PlayerController.SetViewTargetWithBlend` _returnvalue _returnvalue_2 0.0 "VTBlend_Linear" 0.0 false)))

(event `InputAxis|Crouch/FlyDown`
  (params (AxisValue :type "Float (single-precision)"))
  (bind _cabin (`self.Cabin`))
  ;[1 1 1] Movement
  (`PrimitiveComponent.SetPhysicsLinearVelocity` (`/Game/Blueprints/Components/CompParent.Basement` _cabin) (* (`SceneComponent.GetUpVector` (`/Game/Blueprints/Components/Cabin.Camera` _cabin)) (* (`self.Flying Speed`) AxisValue)) true "None"))

(event `InputAxis|ImpulseRight`
  (params (AxisValue :type "Float (single-precision)"))
  (bind _cabin (`self.Cabin`))
  ;[1 1 1] Movement
  (`PrimitiveComponent.SetPhysicsLinearVelocity` (`/Game/Blueprints/Components/CompParent.Basement` _cabin) (* (`SceneComponent.GetRightVector` (`/Game/Blueprints/Components/Cabin.Camera` _cabin)) (* (`self.Flying Speed`) AxisValue)) true "None"))

(event `InputAxis|LookUp / Pitch`
  (params (AxisValue :type "Float (single-precision)"))
  (bind _cabin (`self.Cabin`))
  ;[1 1 1] Rotation
  (`PrimitiveComponent.SetPhysicsAngularVelocity` (`/Game/Blueprints/Components/CompParent.Basement` _cabin) (* (`SceneComponent.GetRightVector` (`/Game/Blueprints/Components/Cabin.Camera` _cabin)) AxisValue) true "None"))

(event `InputAxis|Turn / Yaw`
  (params (AxisValue :type "Float (single-precision)"))
  (bind _cabin (`self.Cabin`))
  ;[1 1 1] Rotation
  (`PrimitiveComponent.SetPhysicsAngularVelocity` (`/Game/Blueprints/Components/CompParent.Basement` _cabin) (* (`SceneComponent.GetUpVector` (`/Game/Blueprints/Components/Cabin.Camera` _cabin)) AxisValue) true "None"))

(event `InputAxis|Roll`
  (params (AxisValue :type "Float (single-precision)"))
  (bind _cabin (`self.Cabin`))
  ;[1 1 1] Rotation
  (`PrimitiveComponent.SetPhysicsAngularVelocity` (`/Game/Blueprints/Components/CompParent.Basement` _cabin) (* (`SceneComponent.GetForwardVector` (`/Game/Blueprints/Components/Cabin.Camera` _cabin)) AxisValue) true "None"))

(fn `UserConstructionScript`)