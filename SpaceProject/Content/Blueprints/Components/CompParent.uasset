(fn ConstructionScript)

(fn SpawnCollision
  (bind _scalevalue (Variables|ConstructionCharacteristics|GetScaleValue))
  (bind _returnvalue (Game|SpawnActorfromClass (Variables|ConstructionCharacteristics|GetCollisionClass) (Transformation|GetActorTransform self) "AlwaysSpawn" 0 0))
  (bind _asccoll_parent (Utilities|Casting|CastToCCollParent _returnvalue)
    (:then
      (bind _output_get (Variables|ConstructionCharacteristics|SetSelfCColl _asccoll_parent))
      (Utilities|FlowControl|Sequence
        (:then_0
          (Variables|/Game/Blueprints/Components/Collisions/CCollParent.CCollParent_C|SetCompOffset _output_get (* _scalevalue (Variables|/Game/Blueprints/Components/Collisions/CCollParent.CCollParent_C|GetCompOffset _output_get)))
          (Variables|/Game/Blueprints/Components/Collisions/CCollParent.CCollParent_C|SetOneSideOffset _output_get (* _scalevalue (Variables|/Game/Blueprints/Components/Collisions/CCollParent.CCollParent_C|GetOneSideOffset _output_get)))
          (Variables|/Game/Blueprints/Components/Collisions/CCollParent.CCollParent_C|SetSelfComp _output_get self))
        (:then_1
          (Class|SceneComponent|Attachto (VehicleSound|GetRootComponent (Variables|ConstructionCharacteristics|GetSelfCColl)) (VehicleSound|GetRootComponent self) "None" "KeepWorldPosition" false)
          (return))))
    (:CastFailed
      (return))))

(fn DestroyCollision
  (Utilities|IsValid (Variables|ConstructionCharacteristics|GetSelfCColl)
    (:Is%20Valid
      (Actor|DestroyActor (Variables|ConstructionCharacteristics|GetSelfCColl))
      (Variables|ConstructionCharacteristics|SetSelfCColl 0))
    (:Is%20Not%20Valid
      _))
  (return))

(fn SetBuildMode
  (params (True :type Boolean))
  (if True
    (if (Variables|ConstructionCharacteristics|GetEditable)
      _
      (else
        (Variables|ConstructionCharacteristics|SetEditable true)
        (CallFunction|SpawnCollision)))
    (elif (Variables|ConstructionCharacteristics|GetEditable)
      (Variables|ConstructionCharacteristics|SetEditable false)
      (CallFunction|DestroyCollision)))
  (return))

(fn Reconstruct
  (params (UpdateVariables :type Boolean) (NewStable :type Boolean) (NewConstructed :type Boolean))
  (bind _array (Utilities|Array|MakeArray 0))
  (bind _array_2 (Utilities|Array|MakeArray 0))
  (bind _basement (Variables|Default|GetBasement))
  (bind _basement_2 (Variables|Default|GetBasement))
  (bind _basement_3 (Variables|Default|GetBasement))
  (if (not UpdateVariables)
    _
    (else
      (Variables|ConstructionCharacteristics|SetStable NewStable)
      (Variables|ConstructionCharacteristics|SetConstructed NewConstructed)))
  (Utilities|FlowControl|Sequence
    (:then_0
      (if (Variables|ConstructionCharacteristics|GetStable)
        (if (Variables|ConstructionCharacteristics|GetConstructed)
          (Development|SetHiddeninGame _basement_2 false false)
          (Collision|SetCollisionEnabled _basement_2 "QueryAndPhysics")
          (Physics|SetSimulatePhysics _basement_2 true)
          (Development|SetHiddeninGame (Variables|Default|GetHologramm) true false)
          (else
            (Development|SetHiddeninGame _basement true false)
            (Physics|SetSimulatePhysics _basement false)
            (Collision|SetCollisionEnabled _basement "NoCollision")
            (Development|SetHiddeninGame (Variables|Default|GetHologramm) false false)))
        (CallFunction|Revalidate true false _array _array)
        (else
          (Physics|SetSimulatePhysics _basement_3 false)
          (Collision|SetCollisionEnabled _basement_3 "NoCollision")
          (CallFunction|Revalidate true false _array_2 _array_2)
          (CallFunction|SetBuildMode false)
          (Utilities|Array|RemoveItem (Variables|CompParent_C|GetChildrenComps (Variables|ConstructionCharacteristics|GetRootCabin)) self)
          (Actor|DestroyActor))))
    (:then_1
      (return))))

(fn Revalidate
  (params (AffectNeighbours :type Boolean) (MakeChainReaction :type Boolean) (ChainExceptions :type Array%20of%20Actor%20Object%20References) (AdditionalIgnore :type Array%20of%20Actor%20Object%20References))
  (bind _validity (Variables|ConstructionCharacteristics|GetValidity))
  (LocalVariables|SetChainExceptions_l ChainExceptions)
  (LocalVariables|SetIgnores AdditionalIgnore)
  (Utilities|FlowControl|Sequence
    (:then_0
      (LocalVariables|SetTempEditability_l (Variables|ConstructionCharacteristics|GetEditable))
      (CallFunction|SetBuildMode true)
      (Utilities|Array|Add (LocalVariables|GetIgnores) self)
      (Utilities|Array|Add (LocalVariables|GetIgnores) (Variables|ConstructionCharacteristics|GetSelfCColl))
      (for _array_element (Actor|GetComponentsByClass (Variables|ConstructionCharacteristics|GetSelfCColl) "/Script/Engine.BoxComponent")
        (bind (_outhit _returnvalue) (Collision|SphereTraceForObjects (Transformation|GetWorldLocation _array_element) (+ (Transformation|GetWorldLocation _array_element) (* (Math|Vector|GetForwardVector _array_element) 20)) (/ (Variables|/Game/Blueprints/Components/Collisions/CCollParent.CCollParent_C|GetOneSideOffset (Variables|ConstructionCharacteristics|GetSelfCColl)) 2.0) (Utilities|Array|MakeArray "ObjectTypeQuery7") false (LocalVariables|GetIgnores) "None" false))
        (if _returnvalue
          (bind _ascomp_parent (Utilities|Casting|CastToCompParent (.HitActor (Collision|BreakHitResult _outhit)))
            (:then
              (if (== (Variables|CompParent_C|GetRootCabin _ascomp_parent) (Variables|ConstructionCharacteristics|GetRootCabin))
                (Utilities|Array|Add (LocalVariables|GetNeighbours_l) _ascomp_parent)
                (Utilities|Array|SetArrayElem _validity (Math|Conversions|ToInteger(Byte) (Utilities|GetObjectName _array_element)) false)
                (else
                  (Utilities|Array|SetArrayElem _validity (Math|Conversions|ToInteger(Byte) (Utilities|GetObjectName _array_element)) true :!label _label))))
            (:CastFailed
              (goto _label)))
          (else
            (Utilities|Array|SetArrayElem (Variables|ConstructionCharacteristics|GetValidity) (Math|Conversions|ToInteger(Byte) (Utilities|GetObjectName _array_element)) true)))))
    (:then_1
      (Utilities|Array|Add (LocalVariables|GetChainExceptions_l) self))
    (:then_2
      (CallFunction|SetBuildMode (LocalVariables|GetTempEditability_l))
      (if AffectNeighbours
        (for _array_element_2 (LocalVariables|GetNeighbours_l)
          (if (not (Utilities|Array|ContainsItem (LocalVariables|GetChainExceptions_l) _array_element_2))
            (CallFunction|Revalidate _array_element_2 MakeChainReaction MakeChainReaction (LocalVariables|GetChainExceptions_l) AdditionalIgnore)))))
    (:then_3
      (return (LocalVariables|GetNeighbours_l)))))